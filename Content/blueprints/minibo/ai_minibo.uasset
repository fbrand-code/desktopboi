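; AI controller for the minibo character that makes it chase the player.
; It caches the possessed bpc_minibo and the first player pawn.
; Every tick it takes the forward vector of the look-at rotation toward the player and passes it to the pawn's Followplayer function.
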(event EventBeginPlay
  (Variables|Default|Setplayer (Game|Player|GetPlayerPawn 0)))

(event EventTick
  (params (DeltaSeconds :type Float%20%28single-precision%29))
  (Default|Followplayer (Variables|Default|GetPossessed%20Pawn) (Math|Vector|GetForwardVector (Math|Rotator|FindLookatRotation (Transformation|GetActorLocation (Variables|Default|GetPossessed%20Pawn)) (Transformation|GetActorLocation (Variables|Default|Getplayer))))))

(event EventPossess
  (params (PossessedPawn :type Pawn%20Object%20Reference))
  (bind _asbpc_minibo (Utilities|Casting|CastTobpc_minibo PossessedPawn))
  (Variables|Default|SetPossessed%20Pawn _asbpc_minibo))

(fn ConstructionScript)