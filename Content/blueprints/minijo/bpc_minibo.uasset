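; Minibo pawn Blueprint that moves along a supplied direction and damages the minijo character on contact.
; Its followplayer event adds movement input only when Canmove0 passes, which returns the inverse of the AcHealth component's Isalive flag.
; When its Hitbox begins overlapping a bpc_minijo's Damagebox specifically, it applies damage to that actor.
; BeginPlay, Tick and actor overlap are unused, so movement relies on followplayer being called.
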(event OnComponentBeginOverlap(hitbox)
  (params (OverlappedComponent :type Primitive%20Component%20Object%20Reference) (OtherActor :type Actor%20Object%20Reference) (OtherComp :type Primitive%20Component%20Object%20Reference) (OtherBodyIndex :type Integer) (bFromSweep :type Boolean) (SweepResult :type Hit%20Result%20Structure%20%28by%20ref%29))
  (bind _asbpc_minijo (Utilities|Casting|CastTobpc_minijo OtherActor))
  (if (== (Variables|/Game/blueprints/minijo/bp_minijo.bp_minijo_C|Getdamagebox _asbpc_minijo) OtherComp)
    (Game|Damage|ApplyDamage _asbpc_minijo 1.0 0 0)))

(event Custom|followplayer
  (params (WorldDirection :type Vector))
  (if (CallFunction|Canmove0)
    (Pawn|Input|AddMovementInput WorldDirection 1.0 false)))

(event EventBeginPlay
  (|CallParentFunction) ; This node is disabled and will not be called.\nDrag off pins to build functionality.
)

(event Collision|EventActorBeginOverlap
  (params (OtherActor :type Actor%20Object%20Reference))
  (|CallParentFunction OtherActor) ; This node is disabled and will not be called.\nDrag off pins to build functionality.
)

(event EventTick
  (params (DeltaSeconds :type Float%20%28single-precision%29))
  (|CallParentFunction DeltaSeconds) ; This node is disabled and will not be called.\nDrag off pins to build functionality.
)

(fn ConstructionScript
  (|CallParentFunction))

(fn Canmove0
  (return (not (Variables|/Game/blueprints/components/ac_health.ac_health_C|Getisalive (Variables|Default|Getac_health)))))