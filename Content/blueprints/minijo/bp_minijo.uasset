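; Player-controllable 2D sprite character with Enhanced Input movement, jump and attack, using PaperZD-style animation.
; Canmove gates input and damage, blocking them while attacking or when AcHealth's Isalive flag is true.
; Damage feeds AcHealth; a true Isalive, apparently meaning dead despite its name, triggers the death animation jump and a cast-gated destroy.
; Attack plays an animation override; separate functions damage overlapping Bp_minijo actors and briefly flash the sprite red.
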(event Custom|spritehit
  (Sprite|SetSpriteColor (Variables|Default|GetSprite) "(R=1.000000,G=0.057292,B=0.119150,A=1.000000)")
  (Utilities|FlowControl|RetriggerableDelay 0.2)
  (Sprite|SetSpriteColor (Variables|Default|GetSprite) "(R=1.000000,G=1.000000,B=1.000000,A=1.000000)"))

(event Input|EnhancedActionEvents|EnhancedInputActionia_jump
  (params (ActionValue :type Boolean) (ElapsedSeconds :type Float%20%28double-precision%29) (TriggeredSeconds :type Float%20%28double-precision%29) (InputAction :type Input%20Action%20Object%20Reference :default "/Game/input/actions/ia_jump.ia_jump"))
  (:Triggered
    (if (CallFunction|Canmove)
      (Character|Jump)))
  (:Completed
    (Character|StopJumping)))

(event Input|EnhancedActionEvents|EnhancedInputActionia_move
  (params (ActionValue :type Vector%202D%20Structure) (ElapsedSeconds :type Float%20%28double-precision%29) (TriggeredSeconds :type Float%20%28double-precision%29) (InputAction :type Input%20Action%20Object%20Reference :default "/Game/input/actions/ia_move.ia_move"))
  (bind (_x _y) (Math|Vector2D|BreakVector2D ActionValue))
  (if (CallFunction|Canmove)
    (Pawn|Input|AddMovementInput "1.000000,0.000000,0.000000" _x false)
    (Pawn|Input|AddMovementInput "0.000000,1.000000,0.000000" _y false)))

(event Input|EnhancedActionEvents|EnhancedInputActionia_attack
  (params (ActionValue :type Boolean) (ElapsedSeconds :type Float%20%28double-precision%29) (TriggeredSeconds :type Float%20%28double-precision%29) (InputAction :type Input%20Action%20Object%20Reference :default "/Game/input/actions/ia_attack.ia_attack"))
  (:Started
    (if (CallFunction|Canmove)
      (|PlayAnimationOverridewithCallbacks (Variables|/Script/PaperZD.PaperZDAnimationComponent|GetAnimInstance (Variables|Default|GetAnimationComponent)) "/Game/blueprints/minijo/AnimSequences/attack.attack" "DefaultSlot" 1.0 0.0
        (:then
          (Variables|Default|Setisattacking true))
        (:OnCompleted
          (Variables|Default|Setisattacking false :!label _label))
        (:OnCancelled
          (goto _label))))))

(event EventBeginPlay
  (bind _asplayer_controller (Utilities|Casting|CastToPlayerController (Pawn|GetController)))
  (Input|AddMappingContext (PlayerController|LocalPlayerSubsystems|GetEnhancedInputLocalPlayerSubsystem _asplayer_controller) "/Game/input/imc.imc" 0 "(bIgnoreAllPressedKeysUntilRelease=True,bForceImmediately=False,bNotifyUserSettings=False)"))

(event Collision|EventActorBeginOverlap
  (params (OtherActor :type Actor%20Object%20Reference)))

(event EventTick
  (params (DeltaSeconds :type Float%20%28single-precision%29)))

(event Game|Damage|EventAnyDamage
  (params (Damage :type Float%20%28single-precision%29) (DamageType :type Damage%20Type%20Object%20Reference) (InstigatedBy :type Controller%20Object%20Reference) (DamageCauser :type Actor%20Object%20Reference))
  (if (CallFunction|Canmove)
    (Default|Damagehealth (Variables|Default|Getac_health) Damage)
    (if (Variables|/Game/blueprints/components/ac_health.ac_health_C|Getisalive (Variables|Default|Getac_health))
      (Class|PaperZDAnimInstance|JumptoNode (Variables|/Script/PaperZD.PaperZDAnimationComponent|GetAnimInstance (Variables|Default|GetAnimationComponent)) "death" "None")
      (Utilities|Casting|CastTobpc_minibo self)
      (Actor|DestroyActor))))

(fn ConstructionScript)

(fn Attackhitbox
  (bind _arrayelement (Utilities|Array|ReverseforEachLoop (Collision|GetOverlappingActors (Variables|Default|Gethitbox) "bp_minijo_C" :!class /Script/Engine.PrimitiveComponent))
    (:LoopBody
      (Game|Damage|ApplyDamage _arrayelement 1.0 0 0))))

(fn Canmove
  (return (and (not (Variables|Default|Getisattacking)) (not (Variables|/Game/blueprints/components/ac_health.ac_health_C|Getisalive (Variables|Default|Getac_health))))))